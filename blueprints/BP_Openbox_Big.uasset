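; BP_Openbox_Big controls a proximity-based Widget that stops showing once the player has visited its location.
; Each Tick measures the distance from the Widget to the player's MyCharacter and shows it only in a band between near and far thresholds while unvisited.
; Coming inside the near threshold hides it and starts a short Delay, after which IsViisited is set, keeping the Widget hidden.
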(event EventBeginPlay)

(event Collision|EventActorBeginOverlap
  (params (OtherActor :type Actor%20Object%20Reference)))

(event EventTick
  (params (DeltaSeconds :type Float%20%28single-precision%29))
  (bind _widget (Variables|Default|GetWidget))
  (bind _asmy_character (Utilities|Casting|CastToMyCharacter (Game|GetPlayerCharacter 0)))
  (if (and (and (< (Math|Vector|Distance(Vector) (Transformation|GetWorldLocation (Variables|Default|GetWidget)) (Transformation|GetActorLocation _asmy_character)) 2e+03) (> (Math|Vector|Distance(Vector) (Transformation|GetWorldLocation (Variables|Default|GetWidget)) (Transformation|GetActorLocation _asmy_character)) 1.8e+02)) (not (Variables|Default|GetisViisited)))
    (Rendering|SetVisibility _widget true true)
    (else
      (Rendering|SetVisibility _widget false true)))
  (if (< (Math|Vector|Distance(Vector) (Transformation|GetWorldLocation (Variables|Default|GetWidget)) (Transformation|GetActorLocation _asmy_character)) 1.8e+02)
    (Utilities|FlowControl|Delay 2.0)
    (Variables|Default|SetisViisited true)))

(fn ConstructionScript)
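; Player HUD that owns the game's UMG widgets and draws per-weapon crosshairs.
; BeginPlay creates all widgets; once the pawn's movie action state is End, DrawHUD syncs their visibility to My_Pers flags each frame.
; Unless the crosshair state is Sniper, NewFunction swaps white or red textures by Regular or Target state.
; The current weapon's ammo type selects the crosshair layout, whose spread grows with camera FOV and player speed.
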(event EventBeginPlay
  ;[0 0.3952 1] INIT WIDGETS
  (bind _returnvalue (UserInterface|CreateWidget "/Game/MyBPs/MY_WIDGETS/PersWidget.PersWidget_C"))
  (bind _output_get (Variables|Default|SetPersWidget _returnvalue))
  (UserInterface|Viewport|AddtoViewport _output_get 0)
  (bind _asmy_pers (Utilities|Casting|CastToMy_Pers (Game|Player|GetPlayerPawn 0)))
  (Class|MyCharacter|SetIsPersWidgetShown _asmy_pers true)
  (bind _returnvalue_2 (UserInterface|CreateWidget "/Game/MyBPs/MY_WIDGETS/WeaponConfigWidget.WeaponConfigWidget_C"))
  (bind _output_get_2 (Variables|Default|SetWeaponWidget _returnvalue_2))
  (UserInterface|Viewport|AddtoViewport _output_get_2 0)
  (Variables|/Script/UMG.Widget|SetVisibility _output_get_2 "Hidden")
  (bind _returnvalue_3 (UserInterface|CreateWidget "/Game/MyBPs/MY_WIDGETS/GameMenuWidget.GameMenuWidget_C"))
  (bind _output_get_3 (Variables|Default|SetGameMenuWidget _returnvalue_3))
  (UserInterface|Viewport|AddtoViewport _output_get_3 0)
  (Variables|/Script/UMG.Widget|SetVisibility _output_get_3 "Hidden")
  (bind _returnvalue_4 (UserInterface|CreateWidget "/Game/MyBPs/MY_WIDGETS/MainMenuWidget.MainMenuWidget_C"))
  (bind _output_get_4 (Variables|Default|SetMainMenuWidget _returnvalue_4))
  (UserInterface|Viewport|AddtoViewport _output_get_4 0)
  (Variables|/Script/UMG.Widget|SetVisibility _output_get_4 "Hidden")
  (bind _returnvalue_5 (UserInterface|CreateWidget "/Game/MyBPs/MY_WIDGETS/SettingsMenuWidget.SettingsMenuWidget_C"))
  (bind _output_get_5 (Variables|Default|SetSettingsMenuWidget _returnvalue_5))
  (UserInterface|Viewport|AddtoViewport _output_get_5 0)
  (Variables|/Script/UMG.Widget|SetVisibility _output_get_5 "Hidden")
  (bind _returnvalue_6 (UserInterface|CreateWidget "/Game/MyBPs/MY_WIDGETS/RespawnWidget.RespawnWidget_C"))
  (bind _output_get_6 (Variables|Default|SetRespawnMenuWidget _returnvalue_6))
  (UserInterface|Viewport|AddtoViewport _output_get_6 0)
  (Variables|/Script/UMG.Widget|SetVisibility _output_get_6 "Hidden"))

(event EventDrawHUD
  (params (SizeX :type Integer) (SizeY :type Integer))
  (bind _scalesmg11 (Variables|Default|GetscaleSMG11))
  (bind _crosshairsize (Variables|Default|GetcrosshairSize))
  (bind _crosshairsize_2 (Variables|Default|GetcrosshairSize))
  (bind _crosshairsize_3 (Variables|Default|GetcrosshairSize))
  (bind _crosshairsize_4 (Variables|Default|GetcrosshairSize))
  (bind _crosshairsize_5 (Variables|Default|GetcrosshairSize))
  (bind _crosshairpistolarcur (Variables|Default|GetcrosshairPistolArCur))
  (bind _gamemenuwidget (Variables|Default|GetGameMenuWidget))
  (bind _mainmenuwidget (Variables|Default|GetMainMenuWidget))
  (bind _weaponwidget (Variables|Default|GetWeaponWidget))
  (bind _perswidget (Variables|Default|GetPersWidget))
  (bind _settingsmenuwidget (Variables|Default|GetSettingsMenuWidget))
  (bind _respawnmenuwidget (Variables|Default|GetRespawnMenuWidget))
  (bind _crosshairsize_6 (Variables|Default|GetcrosshairSize))
  (bind _crosshairsize_7 (Variables|Default|GetcrosshairSize))
  (bind _scalesmg11_2 (Variables|Default|GetscaleSMG11))
  (bind _crosshairsize_8 (Variables|Default|GetcrosshairSize))
  (bind _crosshairsize_9 (Variables|Default|GetcrosshairSize))
  (bind _crosshairsize_10 (Variables|Default|GetcrosshairSize))
  (bind _crosshairsize_11 (Variables|Default|GetcrosshairSize))
  (bind _crosshairsize_12 (Variables|Default|GetcrosshairSize))
  (bind _scalepistol (Variables|Default|GetscalePistol))
  (bind _crosshairsize_13 (Variables|Default|GetcrosshairSize))
  (bind _scalepistol_2 (Variables|Default|GetscalePistol))
  (bind _crosshairsize_14 (Variables|Default|GetcrosshairSize))
  (bind _crosshairsize_15 (Variables|Default|GetcrosshairSize))
  (bind _crosshairsize_16 (Variables|Default|GetcrosshairSize))
  (bind _crosshairsize_17 (Variables|Default|GetcrosshairSize))
  (bind _crosshairsize_18 (Variables|Default|GetcrosshairSize))
  (bind _crosshairsize_19 (Variables|Default|GetcrosshairSize))
  (bind _crosshairsize_20 (Variables|Default|GetcrosshairSize))
  (bind _returnvalue (* _crosshairsize_12 1.7))
  (bind _returnvalue_2 (* _crosshairsize_15 2.3))
  (bind _returnvalue_3 (* _crosshairsize_9 2.3))
  (bind _returnvalue_4 (* _crosshairsize_13 1.7))
  (bind _returnvalue_5 (* _crosshairsize_10 1.2))
  (bind _returnvalue_6 (* _crosshairsize_11 1.2))
  (bind _returnvalue_7 (/ _crosshairsize_14 4.2))
  ;[1 1 1] Prepare Crosshair
  (Variables|Default|SetscreenCenter (Math|Vector2D|MakeVector2D (Math|Conversions|ToFloat(Integer) (/ SizeX 2)) (Math|Conversions|ToFloat(Integer) (/ SizeY 2))))
  (bind _asmy_pers (Utilities|Casting|CastToMy_Pers (Game|Player|GetPlayerPawn 0)))
  (bind _returnvalue_8 (Class|MyCharacter|GetMovieActionState _asmy_pers))
  (if (Utilities|Enum|Equal(Enum) _returnvalue_8 "ES_End")
    (Utilities|FlowControl|Sequence
      (:then_0
        ;[0.03372 0.3245 1] GAME Menu WIDGET ON/OFF
        (bind _returnvalue_9 (Class|MyCharacter|GetIsGameMenuShown _asmy_pers))
        (if _returnvalue_9
          (Variables|/Script/UMG.Widget|SetVisibility _gamemenuwidget "Visible")
          (else
            (Variables|/Script/UMG.Widget|SetVisibility _gamemenuwidget "Hidden"))))
      (:then_1
        ;[0.03372 0.3245 1] WEAPON CONFIG WIDGET ON/OFF
        (bind _returnvalue_10 (Class|MyCharacter|GetIsWeaponConfigure _asmy_pers))
        (if _returnvalue_10
          (Variables|/Script/UMG.Widget|SetVisibility _weaponwidget "Visible")
          (else
            (Variables|/Script/UMG.Widget|SetVisibility _weaponwidget "Hidden"))))
      (:then_2
        (Variables|Default|SetField%20Of%20View (Variables|/Script/Engine.CameraComponent|GetFieldOfView (Variables|/Script/TEST1.MyCharacter|GetmyCamera _asmy_pers)))
        (Variables|Default|SetVelocity (Math|Vector|VectorLength (Transformation|GetVelocity _asmy_pers)))
        (bind _output_get (Variables|Default|SetcrosshairState (Class|MyCharacter|GetCrosshairState _asmy_pers)))
        (if (Utilities|Enum|NotEqual(Enum) _output_get "ES_Sniper")
          ;[1 1 1] Pistol Color Crosshair
          (CallFunction|NewFunction (Variables|Default|GetcrosshairPistolAr) (Variables|Default|GetcrosshairPistolArCur) (Variables|Default|GetcrosshairPistolArR))
          ;[1 1 1] SMG11 Color Crosshair
          (CallFunction|NewFunction (Variables|Default|GetcrosshairSMG11Ar) (Variables|Default|GetcrosshairSMG11ArCur) (Variables|Default|GetcrosshairSMG11ArR))
          ;[1 1 1] AR4 Color Crosshair
          (CallFunction|NewFunction (Variables|Default|GetcrosshairAR4Ar) (Variables|Default|GetcrosshairAR4ArCur) (Variables|Default|GetcrosshairAR4ArR))
          ;[1 1 1] Sniper Color Crosshair
          (CallFunction|NewFunction (Variables|Default|GetcrosshairSniperAr) (Variables|Default|GetcrosshairSniperArCur) (Variables|Default|GetcrosshairSniperArR))
          ;[1 1 1] Minigun Color Crosshair
          (CallFunction|NewFunction (Variables|Default|GetcrosshairMinigunAr) (Variables|Default|GetcrosshairMinigunArCur) (Variables|Default|GetcrosshairMinigunArR))
          (Utilities|IsValid (Variables|/Script/TEST1.MyCharacter|GetcurrentWeapon _asmy_pers)
            (:Is%20Valid
              (switch Utilities|FlowControl|Switch|SwitchonEAmmoType (Variables|/Script/TEST1.MyWeapon|GetammoType (Variables|/Script/TEST1.MyCharacter|GetcurrentWeapon _asmy_pers))
                (:ES_AmmoPistol
                  ;[1 1 1] Pistol Crosshair
                  (Variables|Default|SetdeltaRadiusPistol (/ (/ (Math|Float|Sqrt (+ (Math|Float|Power _crosshairsize_12 2.0) (Math|Float|Power _returnvalue 2.0))) 2.0) (Math|Trig|Sin(Degrees) 6e+01)))
                  (Canvas|DrawTexture (Utilities|Array|Get(acopy) _crosshairpistolarcur) (- (- (.x (Variables|Default|GetscreenCenter)) _crosshairsize_12) (+ (/ (Variables|Default|GetField%20Of%20View) _scalepistol) (/ (Variables|Default|GetVelocity) (Variables|Default|GetVelocityKoef)))) (- (- (.y (Variables|Default|GetscreenCenter)) (Variables|Default|GetdeltaRadiusPistol)) (+ (/ (Variables|Default|GetField%20Of%20View) _scalepistol) (/ (Variables|Default|GetVelocity) (Variables|Default|GetVelocityKoef)))) _crosshairsize_12 _returnvalue 0.0 0.0 1.0 1.0 "(R=1.000000,G=1.000000,B=1.000000,A=1.000000)")
                  (Canvas|DrawTexture (Utilities|Array|Get(acopy) _crosshairpistolarcur 1) (+ (.x (Variables|Default|GetscreenCenter)) (+ (/ (Variables|Default|GetField%20Of%20View) _scalepistol_2) (/ (Variables|Default|GetVelocity) (Variables|Default|GetVelocityKoef)))) (- (- (.y (Variables|Default|GetscreenCenter)) (Variables|Default|GetdeltaRadiusPistol)) (+ (/ (Variables|Default|GetField%20Of%20View) _scalepistol_2) (/ (Variables|Default|GetVelocity) (Variables|Default|GetVelocityKoef)))) _crosshairsize_13 _returnvalue_4 0.0 0.0 1.0 1.0 "(R=1.000000,G=1.000000,B=1.000000,A=1.000000)")
                  (Canvas|DrawTexture (Utilities|Array|Get(acopy) _crosshairpistolarcur 2) (- (.x (Variables|Default|GetscreenCenter)) _crosshairsize_14) (+ (- (+ (.y (Variables|Default|GetscreenCenter)) (- _returnvalue_4 (Variables|Default|GetdeltaRadiusPistol))) _returnvalue_7) (+ (/ (Variables|Default|GetField%20Of%20View) (Variables|Default|GetscalePistol)) (/ (Variables|Default|GetVelocity) (Variables|Default|GetVelocityKoef)))) (* _crosshairsize_14 2.0) _returnvalue_7 0.0 0.0 1.0 1.0 "(R=1.000000,G=1.000000,B=1.000000,A=1.000000)"))
                (:ES_AmmoSMG11
                  ;[1 1 1] SMG11 Crosshair
                  (Variables|Default|SetdeltaRadiusPistol (/ (/ (Math|Float|Sqrt (+ (Math|Float|Power _crosshairsize_10 2.0) (Math|Float|Power _returnvalue_5 2.0))) 2.0) (Math|Trig|Sin(Degrees) 6e+01)))
                  (Canvas|DrawTexture (Utilities|Array|Get(acopy) (Variables|Default|GetcrosshairSMG11ArCur)) (- (- (.x (Variables|Default|GetscreenCenter)) _crosshairsize_10) (+ (/ (Variables|Default|GetField%20Of%20View) _scalesmg11) (/ (Variables|Default|GetVelocity) (Variables|Default|GetVelocityKoef)))) (- (- (.y (Variables|Default|GetscreenCenter)) (Variables|Default|GetdeltaRadiusPistol)) (+ (/ (Variables|Default|GetField%20Of%20View) _scalesmg11) (/ (Variables|Default|GetVelocity) (Variables|Default|GetVelocityKoef)))) _crosshairsize_10 _returnvalue_5 0.0 0.0 1.0 1.0 "(R=1.000000,G=1.000000,B=1.000000,A=1.000000)")
                  (Canvas|DrawTexture (Utilities|Array|Get(acopy) (Variables|Default|GetcrosshairSMG11ArCur) 1) (+ (.x (Variables|Default|GetscreenCenter)) (+ (/ (Variables|Default|GetField%20Of%20View) _scalesmg11_2) (/ (Variables|Default|GetVelocity) (Variables|Default|GetVelocityKoef)))) (- (- (.y (Variables|Default|GetscreenCenter)) (Variables|Default|GetdeltaRadiusPistol)) (+ (/ (Variables|Default|GetField%20Of%20View) _scalesmg11_2) (/ (Variables|Default|GetVelocity) (Variables|Default|GetVelocityKoef)))) _crosshairsize_11 _returnvalue_6 0.0 0.0 1.0 1.0 "(R=1.000000,G=1.000000,B=1.000000,A=1.000000)")
                  (Canvas|DrawTexture (Utilities|Array|Get(acopy) (Variables|Default|GetcrosshairSMG11ArCur) 2) (- (.x (Variables|Default|GetscreenCenter)) (/ _returnvalue_6 2.0)) (+ (.y (Variables|Default|GetscreenCenter)) (+ (/ (Variables|Default|GetField%20Of%20View) (Variables|Default|GetscaleSMG11)) (/ (Variables|Default|GetVelocity) (Variables|Default|GetVelocityKoef)))) (* _returnvalue_6 1.07) (/ (Variables|Default|GetcrosshairSize) 1.2) 0.0 0.0 1.0 1.0 "(R=1.000000,G=1.000000,B=1.000000,A=1.000000)"))
                (:ES_AmmoAR4
                  ;[1 1 1] AR4 Crosshair
                  (Canvas|DrawTexture (Utilities|Array|Get(acopy) (Variables|Default|GetcrosshairAR4ArCur)) (- (.x (Variables|Default|GetscreenCenter)) (+ _crosshairsize_6 (+ (/ (Variables|Default|GetField%20Of%20View) (Variables|Default|GetscaleAR4)) (/ (Variables|Default|GetVelocity) (Variables|Default|GetVelocityKoef))))) (- (.y (Variables|Default|GetscreenCenter)) (/ _crosshairsize_6 2.0)) _crosshairsize_6 _crosshairsize_6 0.0 0.0 1.0 1.0 "(R=1.000000,G=1.000000,B=1.000000,A=1.000000)")
                  (Canvas|DrawTexture (Utilities|Array|Get(acopy) (Variables|Default|GetcrosshairAR4ArCur) 1) (- (.x (Variables|Default|GetscreenCenter)) (/ _crosshairsize 2.0)) (- (.y (Variables|Default|GetscreenCenter)) (+ _crosshairsize (+ (/ (Variables|Default|GetField%20Of%20View) (Variables|Default|GetscaleAR4)) (/ (Variables|Default|GetVelocity) (Variables|Default|GetVelocityKoef))))) _crosshairsize _crosshairsize 0.0 0.0 1.0 1.0 "(R=1.000000,G=1.000000,B=1.000000,A=1.000000)")
                  (Canvas|DrawTexture (Utilities|Array|Get(acopy) (Variables|Default|GetcrosshairAR4ArCur) 2) (+ (.x (Variables|Default|GetscreenCenter)) (+ (/ (Variables|Default|GetField%20Of%20View) (Variables|Default|GetscaleAR4)) (/ (Variables|Default|GetVelocity) (Variables|Default|GetVelocityKoef)))) (- (.y (Variables|Default|GetscreenCenter)) (/ _crosshairsize_8 2.0)) _crosshairsize_8 _crosshairsize_8 0.0 0.0 1.0 1.0 "(R=1.000000,G=1.000000,B=1.000000,A=1.000000)")
                  (Canvas|DrawTexture (Utilities|Array|Get(acopy) (Variables|Default|GetcrosshairAR4ArCur) 3) (- (.x (Variables|Default|GetscreenCenter)) (/ _crosshairsize_7 2.0)) (+ (.y (Variables|Default|GetscreenCenter)) (+ (/ (Variables|Default|GetField%20Of%20View) (Variables|Default|GetscaleAR4)) (/ (Variables|Default|GetVelocity) (Variables|Default|GetVelocityKoef)))) _crosshairsize_7 _crosshairsize_7 0.0 0.0 1.0 1.0 "(R=1.000000,G=1.000000,B=1.000000,A=1.000000)"))
                (:ES_AmmoSniper
                  ;[1 1 1] Sniper Crosshair
                  (Canvas|DrawTexture (Utilities|Array|Get(acopy) (Variables|Default|GetcrosshairSniperArCur)) (- (.x (Variables|Default|GetscreenCenter)) (/ _crosshairsize_3 2.0)) (- (.y (Variables|Default|GetscreenCenter)) (+ _crosshairsize_3 (+ (+ (Variables|Default|GetdeltaRadSniperHex) (/ (Variables|Default|GetField%20Of%20View) (Variables|Default|GetscaleSniperHex))) (/ (Variables|Default|GetVelocity) (Variables|Default|GetVelocityKoef))))) _crosshairsize_2 (* _crosshairsize_2 1.1) 0.0 0.0 1.0 1.0 "(R=1.000000,G=1.000000,B=1.000000,A=1.000000)")
                  (Canvas|DrawTexture (Utilities|Array|Get(acopy) (Variables|Default|GetcrosshairSniperArCur)) (- (.x (Variables|Default|GetscreenCenter)) (+ (* (+ (+ (Variables|Default|GetdeltaRadSniperHex) (/ (Variables|Default|GetField%20Of%20View) (Variables|Default|GetscaleSniperHex))) (/ (Variables|Default|GetVelocity) (Variables|Default|GetVelocityKoef))) (Math|Trig|Cos(Degrees) 3e+01)) (Variables|Default|GetcrosshairSize))) (+ (.y (Variables|Default|GetscreenCenter)) (* (+ (+ (Variables|Default|GetdeltaRadSniperHex) (/ (Variables|Default|GetField%20Of%20View) (Variables|Default|GetscaleSniperHex))) (/ (Variables|Default|GetVelocity) (Variables|Default|GetVelocityKoef))) (Math|Trig|Cos(Degrees) 6e+01))) _crosshairsize_4 (* _crosshairsize_4 1.1) 0.0 0.0 1.0 1.0 "(R=1.000000,G=1.000000,B=1.000000,A=1.000000)")
                  (Canvas|DrawTexture (Utilities|Array|Get(acopy) (Variables|Default|GetcrosshairSniperArCur)) (+ (.x (Variables|Default|GetscreenCenter)) (* (+ (+ (Variables|Default|GetdeltaRadSniperHex) (/ (Variables|Default|GetField%20Of%20View) (Variables|Default|GetscaleSniperHex))) (/ (Variables|Default|GetVelocity) (Variables|Default|GetVelocityKoef))) (Math|Trig|Cos(Degrees) 3e+01))) (+ (.y (Variables|Default|GetscreenCenter)) (* (+ (+ (Variables|Default|GetdeltaRadSniperHex) (/ (Variables|Default|GetField%20Of%20View) (Variables|Default|GetscaleSniperHex))) (/ (Variables|Default|GetVelocity) (Variables|Default|GetVelocityKoef))) (Math|Trig|Cos(Degrees) 6e+01))) _crosshairsize_5 (* _crosshairsize_5 1.1) 0.0 0.0 1.0 1.0 "(R=1.000000,G=1.000000,B=1.000000,A=1.000000)")
                  (Canvas|DrawTexture (Utilities|Array|Get(acopy) (Variables|Default|GetcrosshairSniperArCur) 3) (- (.x (Variables|Default|GetscreenCenter)) (/ _crosshairsize_19 2.0)) (- (+ (.y (Variables|Default|GetscreenCenter)) (+ _crosshairsize_19 (+ (+ (Variables|Default|GetdeltaRadSniperArrow) (/ (Variables|Default|GetField%20Of%20View) (Variables|Default|GetscaleSniperArrow))) (/ (Variables|Default|GetVelocity) (/ (Variables|Default|GetVelocityKoef) 0.5))))) (/ _crosshairsize_17 6.0)) _crosshairsize_17 (* _crosshairsize_17 1.1) 0.0 0.0 1.0 1.0 "(R=1.000000,G=1.000000,B=1.000000,A=1.000000)")
                  (Canvas|DrawTexture (Utilities|Array|Get(acopy) (Variables|Default|GetcrosshairSniperArCur) 1) (- (- (.x (Variables|Default|GetscreenCenter)) (+ (* (+ (+ (Variables|Default|GetdeltaRadSniperArrow) (/ (Variables|Default|GetField%20Of%20View) (Variables|Default|GetscaleSniperArrow))) (/ (Variables|Default|GetVelocity) (/ (Variables|Default|GetVelocityKoef) 0.5))) (Math|Trig|Cos(Degrees) 3e+01)) _crosshairsize_20)) (/ _crosshairsize_18 2.0)) (- (.y (Variables|Default|GetscreenCenter)) (+ _crosshairsize_20 (* (+ (+ (Variables|Default|GetdeltaRadSniperArrow) (/ (Variables|Default|GetField%20Of%20View) (Variables|Default|GetscaleSniperArrow))) (/ (Variables|Default|GetVelocity) (/ (Variables|Default|GetVelocityKoef) 0.5))) (Math|Trig|Cos(Degrees) 6e+01)))) _crosshairsize_18 (* _crosshairsize_18 1.1) 0.0 0.0 1.0 1.0 "(R=1.000000,G=1.000000,B=1.000000,A=1.000000)")
                  (Canvas|DrawTexture (Utilities|Array|Get(acopy) (Variables|Default|GetcrosshairSniperArCur) 2) (+ (+ (.x (Variables|Default|GetscreenCenter)) (* (+ (+ (Variables|Default|GetdeltaRadSniperArrow) (/ (Variables|Default|GetField%20Of%20View) (Variables|Default|GetscaleSniperArrow))) (/ (Variables|Default|GetVelocity) (/ (Variables|Default|GetVelocityKoef) 0.5))) (Math|Trig|Cos(Degrees) 3e+01))) (/ _crosshairsize_16 2.0)) (- (.y (Variables|Default|GetscreenCenter)) (+ _crosshairsize_16 (* (+ (+ (Variables|Default|GetdeltaRadSniperArrow) (/ (Variables|Default|GetField%20Of%20View) (Variables|Default|GetscaleSniperArrow))) (/ (Variables|Default|GetVelocity) (/ (Variables|Default|GetVelocityKoef) 0.5))) (Math|Trig|Cos(Degrees) 6e+01)))) _crosshairsize_16 (* _crosshairsize_16 1.1) 0.0 0.0 1.0 1.0 "(R=1.000000,G=1.000000,B=1.000000,A=1.000000)"))
                (:ES_AmmoMinigun
                  ;[1 1 1] Minigun Crosshair
                  (Canvas|DrawTexture (Utilities|Array|Get(acopy) (Variables|Default|GetcrosshairMinigunArCur)) (- (.x (Variables|Default|GetscreenCenter)) (+ _crosshairsize_15 (+ (/ (Variables|Default|GetField%20Of%20View) (Variables|Default|GetscaleMinigun)) (/ (Variables|Default|GetVelocity) (Variables|Default|GetVelocityKoef))))) (- (.y (Variables|Default|GetscreenCenter)) (/ _returnvalue_2 2.0)) _crosshairsize_15 _returnvalue_2 0.0 0.0 1.0 1.0 "(R=1.000000,G=1.000000,B=1.000000,A=1.000000)")
                  (Canvas|DrawTexture (Utilities|Array|Get(acopy) (Variables|Default|GetcrosshairMinigunArCur) 1) (+ (.x (Variables|Default|GetscreenCenter)) (+ (/ (Variables|Default|GetField%20Of%20View) (Variables|Default|GetscaleMinigun)) (/ (Variables|Default|GetVelocity) (Variables|Default|GetVelocityKoef)))) (- (.y (Variables|Default|GetscreenCenter)) (/ _returnvalue_3 2.0)) _crosshairsize_9 _returnvalue_3 0.0 0.0 1.0 1.0 "(R=1.000000,G=1.000000,B=1.000000,A=1.000000)")))))))
      (:then_3
        ;[0.03372 0.3245 1] MAIN Menu WIDGET ON/OFF
        (bind _returnvalue_11 (Class|MyCharacter|GetIsMainMenuShown _asmy_pers))
        (if _returnvalue_11
          (Variables|/Script/UMG.Widget|SetVisibility _mainmenuwidget "Visible")
          (else
            (Variables|/Script/UMG.Widget|SetVisibility _mainmenuwidget "Hidden"))))
      (:then_4
        ;[0.03372 0.3245 1] SETTING Menu WIDGET ON/OFF
        (bind _returnvalue_12 (Class|MyCharacter|GetIsSettingsMenuShown _asmy_pers))
        (if _returnvalue_12
          (Variables|/Script/UMG.Widget|SetVisibility _settingsmenuwidget "Visible")
          (else
            (Variables|/Script/UMG.Widget|SetVisibility _settingsmenuwidget "Hidden"))))
      (:then_5
        ;[0.03372 0.3245 1] PERS WIDGET ON/OFF
        (bind _returnvalue_13 (Class|MyCharacter|GetIsPersWidgetShown _asmy_pers))
        (if _returnvalue_13
          (Variables|/Script/UMG.Widget|SetVisibility _perswidget "Visible")
          (else
            (Variables|/Script/UMG.Widget|SetVisibility _perswidget "Hidden"))))
      (:then_6
        ;[0.03372 0.3245 1] SETTING Menu WIDGET ON/OFF
        (bind _returnvalue_14 (Class|MyCharacter|GetIsRespawnMenuShown _asmy_pers))
        (if _returnvalue_14
          (Variables|/Script/UMG.Widget|SetVisibility _respawnmenuwidget "Visible")
          (else
            (Variables|/Script/UMG.Widget|SetVisibility _respawnmenuwidget "Hidden")))))))

(fn ConstructionScript)

(fn NewFunction
  (params (White :type Array%20of%20Texture%20Object%20References) (Current :type Array%20of%20Texture%20Object%20References) (Red :type Array%20of%20Texture%20Object%20References))
  (Utilities|Array|Clear Current)
  (switch Utilities|FlowControl|Switch|SwitchonEHUDAimState (Variables|Default|GetcrosshairState)
    (:ES_Regular
      (for _array_element White
        (Utilities|Array|Add Current _array_element)))
    (:ES_Target
      (for _array_element_2 Red
        (Utilities|Array|Add Current _array_element_2)))))